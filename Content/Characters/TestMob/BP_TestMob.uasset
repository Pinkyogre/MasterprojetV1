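; BP_TestMob is a test mob that triggers an animation when the player comes within its sphere.
; A sphere overlap by the player pawn sets IsTrigger and runs Verification, which sends a LancerAnim message to AcAnimation and prints the skeletal mesh location.
; BeginPlay also prints that location for debugging.
; Its own LancerAnim event is empty, IsTrigger is never reset here, and a Hello print is left unconnected.
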(event OnComponentBeginOverlap(Sphere)
  (params (OverlappedComponent :type Primitive%20Component%20Object%20Reference) (OtherActor :type Actor%20Object%20Reference) (OtherComp :type Primitive%20Component%20Object%20Reference) (OtherBodyIndex :type Integer) (bFromSweep :type Boolean) (SweepResult :type Hit%20Result%20Structure%20%28by%20ref%29))
  (if (Collision|IsOverlappingActor (Variables|Default|GetSphere) (Game|Player|GetPlayerPawn 0) :!class /Script/Engine.PrimitiveComponent)
    (Variables|Default|SetIsTrigger? true)
    (CallFunction|Verification)))

(event EventVerification
  (if (Variables|Default|GetIsTrigger?)
    (Class|CustomEventInterface|LancerAnim(Message) (Variables|Default|Getac_Animation))
    (Development|PrintString (Utilities|String|ToString(Vector) (.location (Transformation|GetWorldTransform (Variables|Default|GetSkeletalMesh)))) true true "(R=0.000000,G=0.660000,B=1.000000,A=1.000000)" 1e+01)))

(event EventBeginPlay
  (Development|PrintString (Utilities|String|ToString(Vector) (.location (Transformation|GetWorldTransform (Variables|Default|GetSkeletalMesh)))) true true "(R=0.000000,G=0.660000,B=1.000000,A=1.000000)" 1e+01))

(event EventLancerAnim)

(fn ConstructionScript)