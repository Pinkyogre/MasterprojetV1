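; Component that starts its owning BP_C_NPC1 chasing the player and switches on its walking animation.
; The LancerAnim event issues AI MoveTo toward the third-person player pawn, then immediately sets IsWalking on the mesh's ABP_Mutant, with nothing clearing it.
; BeginPlay is empty and no live node here calls LancerAnim; leftover direct-animation, montage and delay experiments are disconnected.
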(event EventBeginPlay)

(event EventLancerAnim
  (bind _asbp_c_npc1 (Utilities|Casting|CastToBP_C_NPC1 (Components|GetOwner)))
  (bind _asbp_third_person_character (Utilities|Casting|CastToBP_ThirdPersonCharacter (Game|Player|GetPlayerPawn 0)))
  (AI|AIMoveTo _asbp_c_npc1 "0, 0, 0" _asbp_third_person_character 5.0 false
    (:then
      (bind _asabp_mutant (Utilities|Casting|CastToABP_Mutant (Components|SkeletalMesh|GetAnimInstance (Variables|/Script/Engine.Character|GetMesh _asbp_c_npc1))))
      (Variables|/Game/Characters/NPC/ABP_Mutant.ABP_Mutant_C|SetbIsWalking _asabp_mutant true))))