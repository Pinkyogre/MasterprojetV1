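; Melee NPC character in three variants, with NPCChoice selecting its mesh and Mutant, Warrok or CH04 AnimBP.
; A sphere overlap starts AI pursuit and leaving it sends the NPC home, while a Tick distance check triggers punch montages and fire effects.
; Hand-collision overlaps trade damage with the player, casting to each AnimBP to set state flags.
; On death it spawns loot nearby: random NFT or pickup, always NFT for CH04.
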(event OnComponentBeginOverlap(Capsule)
  (params (OverlappedComponent :type Primitive%20Component%20Object%20Reference) (OtherActor :type Actor%20Object%20Reference) (OtherComp :type Primitive%20Component%20Object%20Reference) (OtherBodyIndex :type Integer) (bFromSweep :type Boolean) (SweepResult :type Hit%20Result%20Structure%20%28by%20ref%29))
  ;[0 0 0 1 35] NPC reaction to punch
  (bind _asbp_third_person_character (Utilities|Casting|CastToBP_ThirdPersonCharacter OtherActor))
  (Variables|Default|SetbIsOverlapCapsule true)
  (if (Variables|/Game/ThirdPerson/Blueprints/BP_ThirdPersonCharacter.BP_ThirdPersonCharacter_C|GetisPunching? _asbp_third_person_character)
    (if (Class|PrimitiveComponent|IsOverlappingComponent (Variables|Collision|GetCapsuleComponent) (Variables|/Game/ThirdPerson/Blueprints/BP_ThirdPersonCharacter.BP_ThirdPersonCharacter_C|GetRHand%20Box%20Collision _asbp_third_person_character))
      (bind _asabp_mutant (Utilities|Casting|CastToABP_Mutant (Variables|Default|GetAnimInstance))
        (:then
          (Variables|/Game/Characters/NPC/Mutant/ABP_Mutant.ABP_Mutant_C|SetbIsReaction _asabp_mutant true))
        (:CastFailed
          (bind _asabp_warrok (Utilities|Casting|CastToABP_Warrok (Variables|Default|GetAnimInstance))
            (:then
              (Variables|/Game/Characters/NPC/Dwarf/ABP_Warrok.ABP_Warrok_C|SetbIsReaction _asabp_warrok true))
            (:CastFailed
              (bind _asabp_ch04 (Utilities|Casting|CastToABP_CH04 (Variables|Default|GetAnimInstance)))
              (Variables|/Game/Characters/NPC/CH04/ABP_CH04.ABP_CH04_C|SetbIsReaction _asabp_ch04 true)))))
      (Utilities|FlowControl|Delay 0.7)
      (bind _asabp_mutant_2 (Utilities|Casting|CastToABP_Mutant (Variables|Default|GetAnimInstance))
        (:then
          (Variables|/Game/Characters/NPC/Mutant/ABP_Mutant.ABP_Mutant_C|SetbIsReaction _asabp_mutant_2 false)
          (Variables|/Game/Characters/NPC/Mutant/ABP_Mutant.ABP_Mutant_C|SetbIsWalking _asabp_mutant_2 true))
        (:CastFailed
          (bind _asabp_warrok_2 (Utilities|Casting|CastToABP_Warrok (Variables|Default|GetAnimInstance))
            (:then
              (Variables|/Game/Characters/NPC/Dwarf/ABP_Warrok.ABP_Warrok_C|SetbIsReaction _asabp_warrok_2 false)
              (Variables|/Game/Characters/NPC/Dwarf/ABP_Warrok.ABP_Warrok_C|SetbIsWalking _asabp_warrok_2 true))
            (:CastFailed
              (bind _asabp_ch04_2 (Utilities|Casting|CastToABP_CH04 (Variables|Default|GetAnimInstance)))
              (Variables|/Game/Characters/NPC/CH04/ABP_CH04.ABP_CH04_C|SetbIsReaction _asabp_ch04_2 false)
              (Variables|/Game/Characters/NPC/CH04/ABP_CH04.ABP_CH04_C|SetbIsWalking _asabp_ch04_2 true)))))
      (AI|AIMoveTo self "0, 0, 0" (Variables|Default|GetTPCref) 5.0 false
        (:then
          (CallFunction|ByeLife))))))

(event OnComponentEndOverlap(Sphere)
  (params (OverlappedComponent :type Primitive%20Component%20Object%20Reference) (OtherActor :type Actor%20Object%20Reference) (OtherComp :type Primitive%20Component%20Object%20Reference) (OtherBodyIndex :type Integer))
  ;[0 0 0 1 35] Stop Overlap go back to Idle
  (Utilities|Casting|CastToBP_ThirdPersonCharacter OtherActor)
  (Variables|Default|SetIsOverlapSphere false)
  (AI|AIMoveTo self (Variables|Default|GetWorldLocation) 0 5.0 false
    (:OnSuccess
      (bind _asabp_mutant (Utilities|Casting|CastToABP_Mutant (Variables|Default|GetAnimInstance))
        (:then
          (Variables|/Game/Characters/NPC/Mutant/ABP_Mutant.ABP_Mutant_C|SetbIsWalking _asabp_mutant false)
          (Variables|/Game/Characters/NPC/Mutant/ABP_Mutant.ABP_Mutant_C|SetbIsReaction _asabp_mutant false))
        (:CastFailed
          (bind _asabp_warrok (Utilities|Casting|CastToABP_Warrok (Variables|Default|GetAnimInstance))
            (:then
              (Variables|/Game/Characters/NPC/Dwarf/ABP_Warrok.ABP_Warrok_C|SetbIsWalking _asabp_warrok false)
              (Variables|/Game/Characters/NPC/Dwarf/ABP_Warrok.ABP_Warrok_C|SetbIsReaction _asabp_warrok false))
            (:CastFailed
              (bind _asabp_ch04 (Utilities|Casting|CastToABP_CH04 (Variables|Default|GetAnimInstance)))
              (Variables|/Game/Characters/NPC/CH04/ABP_CH04.ABP_CH04_C|SetbIsWalking _asabp_ch04 false)
              (Variables|/Game/Characters/NPC/CH04/ABP_CH04.ABP_CH04_C|SetbIsReaction _asabp_ch04 false))))))))

(event OnComponentBeginOverlap(RhandBoxCollision)
  (params (OverlappedComponent :type Primitive%20Component%20Object%20Reference) (OtherActor :type Actor%20Object%20Reference) (OtherComp :type Primitive%20Component%20Object%20Reference) (OtherBodyIndex :type Integer) (bFromSweep :type Boolean) (SweepResult :type Hit%20Result%20Structure%20%28by%20ref%29))
  ;[0 0 0 1 35] TPC Loosing Life
  (bind _asbp_third_person_character (Utilities|Casting|CastToBP_ThirdPersonCharacter OtherActor))
  (Variables|Default|SetbIsOverlapCapsule true)
  (if (Variables|Default|GetIsPunchingNPC)
    (if (Class|PrimitiveComponent|IsOverlappingComponent (Variables|/Script/Engine.Character|GetCapsuleComponent _asbp_third_person_character) (Variables|Default|GetRhand%20Box%20Collision))
      (bind _asbp_third_person_character_2 (Utilities|Casting|CastToBP_ThirdPersonCharacter (Game|Player|GetPlayerPawn 0)))
      (Variables|/Game/ThirdPerson/Blueprints/BP_ThirdPersonCharacter.BP_ThirdPersonCharacter_C|SetPv _asbp_third_person_character_2 (- (Variables|/Game/ThirdPerson/Blueprints/BP_ThirdPersonCharacter.BP_ThirdPersonCharacter_C|GetPv _asbp_third_person_character_2) 1e+01)))))

(event OnComponentHit(CapsuleComponent)
  (params (HitComponent :type Primitive%20Component%20Object%20Reference) (OtherActor :type Actor%20Object%20Reference) (OtherComp :type Primitive%20Component%20Object%20Reference) (NormalImpulse :type Vector :default "0, 0, 0") (Hit :type Hit%20Result%20Structure%20%28by%20ref%29))
  ;[0 0 0 1 35] If collision between NPC and TPC
  (Utilities|Casting|CastToBP_ThirdPersonCharacter OtherActor)
  (bind _asabp_mutant (Utilities|Casting|CastToABP_Mutant (Variables|Default|GetAnimInstance))
    (:then
      (Variables|/Game/Characters/NPC/Mutant/ABP_Mutant.ABP_Mutant_C|SetbIsWalking _asabp_mutant false)
      (Variables|/Game/Characters/NPC/Mutant/ABP_Mutant.ABP_Mutant_C|SetbIsPunching _asabp_mutant true))
    (:CastFailed
      (bind _asabp_warrok (Utilities|Casting|CastToABP_Warrok (Variables|Default|GetAnimInstance))
        (:then
          (Variables|/Game/Characters/NPC/Dwarf/ABP_Warrok.ABP_Warrok_C|SetbIsWalking _asabp_warrok false)
          (Variables|/Game/Characters/NPC/Dwarf/ABP_Warrok.ABP_Warrok_C|SetbIsPunching _asabp_warrok true))
        (:CastFailed
          (bind _asabp_ch04 (Utilities|Casting|CastToABP_CH04 (Variables|Default|GetAnimInstance)))
          (Variables|/Game/Characters/NPC/CH04/ABP_CH04.ABP_CH04_C|SetbIsWalking _asabp_ch04 false)
          (Variables|/Game/Characters/NPC/CH04/ABP_CH04.ABP_CH04_C|SetbIsPunching _asabp_ch04 true))))))

(event OnComponentBeginOverlap(Sphere)
  (params (OverlappedComponent :type Primitive%20Component%20Object%20Reference) (OtherActor :type Actor%20Object%20Reference) (OtherComp :type Primitive%20Component%20Object%20Reference) (OtherBodyIndex :type Integer) (bFromSweep :type Boolean) (SweepResult :type Hit%20Result%20Structure%20%28by%20ref%29))
  ;[0 0 0 1 35] Overlap Sphere NPC start walking toward TPC
  (Utilities|Casting|CastToBP_ThirdPersonCharacter OtherActor)
  (Variables|Default|SetIsOverlapSphere true)
  (bind _asabp_mutant (Utilities|Casting|CastToABP_Mutant (Variables|Default|GetAnimInstance))
    (:then
      (Variables|/Game/Characters/NPC/Mutant/ABP_Mutant.ABP_Mutant_C|SetbIsWalking _asabp_mutant true)
      (Variables|/Game/Characters/NPC/Mutant/ABP_Mutant.ABP_Mutant_C|SetbIsReaction _asabp_mutant false))
    (:CastFailed
      (bind _asabp_warrok (Utilities|Casting|CastToABP_Warrok (Variables|Default|GetAnimInstance))
        (:then
          (Variables|/Game/Characters/NPC/Dwarf/ABP_Warrok.ABP_Warrok_C|SetbIsWalking _asabp_warrok true)
          (Variables|/Game/Characters/NPC/Dwarf/ABP_Warrok.ABP_Warrok_C|SetbIsReaction _asabp_warrok false))
        (:CastFailed
          (bind _asabp_ch04 (Utilities|Casting|CastToABP_CH04 (Variables|Default|GetAnimInstance)))
          (Variables|/Game/Characters/NPC/CH04/ABP_CH04.ABP_CH04_C|SetbIsWalking _asabp_ch04 true)
          (Variables|/Game/Characters/NPC/CH04/ABP_CH04.ABP_CH04_C|SetbIsReaction _asabp_ch04 false)))))
  (AI|AIMoveTo self "0, 0, 0" (Variables|Default|GetTPCref) 5.0 false))

(event Custom|Drop%20Loot
  (bind _returnvalue (Transformation|GetActorLocation))
  ;[0 0 0 1 35] Drop Loot when ennemy dies
  (bind _outhit (Collision|LineTraceByChannel _returnvalue (- _returnvalue "0,0,200.000000") "TraceTypeQuery1" false (Utilities|Array|MakeArray (Game|GetPlayerCharacter 0)) "None"))
  (Utilities|Casting|CastToABP_Mutant (Variables|Default|GetAnimInstance)
    (:then
      (switch int (Math|Random|RandomIntegerinRange 0 9) :!label _label
        (:Default
          (bind _output_get (Variables|Default|SetFinalRandom 2)))
        (:0
          (Variables|Default|SetFinalRandom 0))
        (:1
          (Variables|Default|SetFinalRandom 1 :!label _label_2))
        (:2
          (goto _label_2))
        (:3
          (goto _label_2))
        (:4
          (goto _label_2))
        (:5
          (goto _label_2))
        (:6
          (goto _label_2))
        (:7
          (goto _label_2))
        (:8
          (goto _label_2))
        (:9
          (goto _label_2)))
      (Game|SpawnActorfromClass (Utilities|Select :Index _output_get :Option%200 "/Game/NFT/BP_NFT.BP_NFT_C" :Option%201 "/Game/InventorySystem/ProjectExample/Blueprints/BP_Pickup.BP_Pickup_C") (Math|Transform|MakeTransform (.RandomLocation (AI|Navigation|GetRandomReachablePointinRadius (.Location (Collision|BreakHitResult _outhit)) 2e+02 0 0)) (Math|Rotator|MakeRotator 0.0 0.0 (Math|Random|RandomFloatinRange 0.0 3.6e+02))) "AdjustIfPossibleButAlwaysSpawn" 0 0))
    (:CastFailed
      (Utilities|Casting|CastToABP_Warrok (Variables|Default|GetAnimInstance)
        (:then
          (goto _label))
        (:CastFailed
          (Utilities|Casting|CastToABP_CH04 (Variables|Default|GetAnimInstance))
          (Game|SpawnActorfromClass "/Game/NFT/BP_NFT.BP_NFT_C" (Math|Transform|MakeTransform (.RandomLocation (AI|Navigation|GetRandomReachablePointinRadius (.Location (Collision|BreakHitResult _outhit)) 2e+02 0 0)) (Math|Rotator|MakeRotator 0.0 0.0 (Math|Random|RandomFloatinRange 0.0 3.6e+02))) "AdjustIfPossibleButAlwaysSpawn" 0 0))))))

(event Custom|ByeLife
  ;[0 0 0 1 35] NPC Loosing Life and Dying
  (Variables|Default|SetPV (- (Variables|Default|GetPV) 1e+01))
  (if (<= (Variables|Default|GetPV) 0.0)
    (bind _asabp_mutant (Utilities|Casting|CastToABP_Mutant (Variables|Default|GetAnimInstance))
      (:then
        (Variables|/Game/Characters/NPC/Mutant/ABP_Mutant.ABP_Mutant_C|SetbIsDying _asabp_mutant true))
      (:CastFailed
        (bind _asabp_warrok (Utilities|Casting|CastToABP_Warrok (Variables|Default|GetAnimInstance))
          (:then
            (Variables|/Game/Characters/NPC/Dwarf/ABP_Warrok.ABP_Warrok_C|SetbIsDying _asabp_warrok true))
          (:CastFailed
            (bind _asabp_ch04 (Utilities|Casting|CastToABP_CH04 (Variables|Default|GetAnimInstance)))
            (Variables|/Game/Characters/NPC/CH04/ABP_CH04.ABP_CH04_C|SetbIsDying _asabp_ch04 true)))))
    (Components|Movement|StopMovementImmediately (Variables|Character|GetCharacterMovement))
    (Variables|Default|SetIsOverlapSphere false)
    (Utilities|FlowControl|Delay 5.0)
    (Actor|DestroyActor)
    (CallFunction|DropLoot)))

(event EventBeginPlay
  ;[0 0 0 1 35] Begin Play
  (Components|Animation|PlayAnimation (Variables|Character|GetMesh) "/Game/Characters/NPC/Mutant/Animation/Mutant_Breathing_Idle.Mutant_Breathing_Idle" true)
  (bind _asbp_third_person_character (Utilities|Casting|CastToBP_ThirdPersonCharacter (Game|Player|GetPlayerPawn 0)))
  (Utilities|IsValid _asbp_third_person_character
    (:Is%20Valid
      (Variables|Default|SetTPCref _asbp_third_person_character)
      (Variables|Default|SetWorldLocation (Transformation|GetWorldLocation (Variables|Character|GetMesh)))
      (Class|SkeletalMeshComponent|SetAnimClass (Variables|Character|GetMesh) (Utilities|Select :Index (Variables|Default|GetNPCChoice) :NewEnumerator0 "/Game/Characters/NPC/Mutant/ABP_Mutant.ABP_Mutant_C" :NewEnumerator1 "/Game/Characters/NPC/Dwarf/ABP_Warrok.ABP_Warrok_C" :NewEnumerator2 "/Game/Characters/NPC/CH04/ABP_CH04.ABP_CH04_C"))
      (Variables|Default|SetAnimInstance (Components|SkeletalMesh|GetAnimInstance (Variables|Character|GetMesh)))
      (Variables|Default|SetIsOverlapSphere false))))

(event EventTick
  (params (DeltaSeconds :type Float%20%28single-precision%29))
  ;[0 0 0 1 35] NPC Punch TPC when in range
  (Utilities|FlowControl|Sequence
    (:then_0
      (if (< (Math|Float|Round (Transformation|GetDistanceTo (Variables|Default|GetTPCref) self)) 200)
        (Utilities|FlowControl|DoOnce false :!label _label
          (:Completed
            (Components|Activation|Activate (Variables|Default|GetP_Fire) false)
            (Components|Activation|Activate (Variables|Default|GetP_FireSecond) false)
            (Variables|Default|SetbIsDistance true)
            (bind _asabp_mutant (Utilities|Casting|CastToABP_Mutant (Variables|Default|GetAnimInstance))
              (:then
                (Variables|/Game/Characters/NPC/Mutant/ABP_Mutant.ABP_Mutant_C|SetbIsWalking _asabp_mutant true)
                (Animation|Montage|MontagePlay (Variables|Default|GetAnimInstance) "/Game/Characters/NPC/Mutant/Animation/Mutant_Punch_Montage.Mutant_Punch_Montage" 1.0 "MontageLength" 0.0 true))
              (:CastFailed
                (bind _asabp_warrok (Utilities|Casting|CastToABP_Warrok (Variables|Default|GetAnimInstance))
                  (:then
                    (Variables|/Game/Characters/NPC/Dwarf/ABP_Warrok.ABP_Warrok_C|SetbIsWalking _asabp_warrok true)
                    (Animation|Montage|MontagePlay (Variables|Default|GetAnimInstance) "/Game/Characters/NPC/Dwarf/Animation/Punch_Montage.Punch_Montage" 1.0 "MontageLength" 0.0 true))
                  (:CastFailed
                    (bind _asabp_ch04 (Utilities|Casting|CastToABP_CH04 (Variables|Default|GetAnimInstance)))
                    (Variables|/Game/Characters/NPC/CH04/ABP_CH04.ABP_CH04_C|SetbIsWalking _asabp_ch04 true)
                    (Animation|Montage|MontagePlay (Variables|Default|GetAnimInstance) "/Game/Characters/NPC/CH04/Animation/Punch_Montage.Punch_Montage" 1.0 "MontageLength" 0.0 true)))))
            (AI|AIMoveTo self "0, 0, 0" (Variables|Default|GetTPCref) 5.0 false
              (:then
                (Variables|Default|SetIsPunchingNPC true)))))
        (else
          (Utilities|FlowControl|Sequence
            (:then_0
              (goto _label Reset))
            (:then_1
              (Components|Activation|Deactivate (Variables|Default|GetP_Fire))
              (Components|Activation|Deactivate (Variables|Default|GetP_FireSecond))
              (Variables|Default|SetbIsDistance false)
              (bind _asabp_mutant_2 (Utilities|Casting|CastToABP_Mutant (Variables|Default|GetAnimInstance))
                (:then
                  (Variables|/Game/Characters/NPC/Mutant/ABP_Mutant.ABP_Mutant_C|SetbIsPunching _asabp_mutant_2 false)
                  (Variables|Default|SetIsPunchingNPC false)
                  (if (Variables|Default|GetIsOverlapSphere)
                    (Variables|/Game/Characters/NPC/Mutant/ABP_Mutant.ABP_Mutant_C|SetbIsWalking _asabp_mutant_2 true)
                    (AI|AIMoveTo self "0, 0, 0" (Variables|Default|GetTPCref) 5.0 false :!label _label_2)))
                (:CastFailed
                  (bind _asabp_warrok_2 (Utilities|Casting|CastToABP_Warrok (Variables|Default|GetAnimInstance))
                    (:then
                      (Variables|/Game/Characters/NPC/Dwarf/ABP_Warrok.ABP_Warrok_C|SetbIsPunching _asabp_warrok_2 false)
                      (Variables|Default|SetIsPunchingNPC false)
                      (if (Variables|Default|GetIsOverlapSphere)
                        (Variables|/Game/Characters/NPC/Dwarf/ABP_Warrok.ABP_Warrok_C|SetbIsWalking _asabp_warrok_2 true)
                        (goto _label_2)))
                    (:CastFailed
                      (bind _asabp_ch04_2 (Utilities|Casting|CastToABP_CH04 (Variables|Default|GetAnimInstance)))
                      (Variables|/Game/Characters/NPC/CH04/ABP_CH04.ABP_CH04_C|SetbIsPunching _asabp_ch04_2 false)
                      (Variables|Default|SetIsPunchingNPC false)
                      (if (Variables|Default|GetIsOverlapSphere)
                        (Variables|/Game/Characters/NPC/CH04/ABP_CH04.ABP_CH04_C|SetbIsWalking _asabp_ch04_2 true)
                        (goto _label_2)))))))))))))

(fn ConstructionScript
  (Class|SkinnedMeshComponent|SetSkeletalMesh (Variables|Character|GetMesh) (Utilities|Array|Get(acopy) (Variables|Default|GetListeNPC) (Math|Conversions|ToInteger(Byte) (Variables|Default|GetNPCChoice))) true))