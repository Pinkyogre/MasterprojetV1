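; Melee NPC character whose mesh and anim class follow NPCChoice, though its behavior requires an ABP_Mutant instance.
; Sphere overlap starts an AIMoveTo chase of the player and exit walks it home, while a Tick distance check triggers the punch montage.
; Hand-box overlaps exchange damage with BP_ThirdPersonCharacter, with only debug prints when player health runs out.
; At zero health the NPC drops a random pickup or NFT nearby, then destroys itself.
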(event OnComponentBeginOverlap(Capsule)
  (params (OverlappedComponent :type Primitive%20Component%20Object%20Reference) (OtherActor :type Actor%20Object%20Reference) (OtherComp :type Primitive%20Component%20Object%20Reference) (OtherBodyIndex :type Integer) (bFromSweep :type Boolean) (SweepResult :type Hit%20Result%20Structure%20%28by%20ref%29))
  ;[0 0 0 1 35] NPC reaction to punch
  (bind _asbp_third_person_character (Utilities|Casting|CastToBP_ThirdPersonCharacter OtherActor))
  (Variables|Default|SetbIsOverlapCapsule true)
  (if (Variables|/Game/ThirdPerson/Blueprints/BP_ThirdPersonCharacter.BP_ThirdPersonCharacter_C|GetisPunching? _asbp_third_person_character)
    (if (Class|PrimitiveComponent|IsOverlappingComponent (Variables|Default|GetCapsule) (Variables|/Game/ThirdPerson/Blueprints/BP_ThirdPersonCharacter.BP_ThirdPersonCharacter_C|GetRHand%20Box%20Collision _asbp_third_person_character))
      (bind _asabp_mutant (Utilities|Casting|CastToABP_Mutant (Variables|Default|GetAnimInstance)))
      (Variables|/Game/Characters/NPC/ABP_Mutant.ABP_Mutant_C|SetbIsReaction _asabp_mutant true)
      (Utilities|FlowControl|Delay 0.7)
      (bind _asabp_mutant_2 (Utilities|Casting|CastToABP_Mutant (Variables|Default|GetAnimInstance)))
      (Variables|/Game/Characters/NPC/ABP_Mutant.ABP_Mutant_C|SetbIsReaction _asabp_mutant_2 false)
      (Variables|/Game/Characters/NPC/ABP_Mutant.ABP_Mutant_C|SetbIsWalking _asabp_mutant_2 true)
      (AI|AIMoveTo self "0, 0, 0" (Variables|Default|GetTPCref) 5.0 false
        (:then
          (CallFunction|ByeLife))))))

(event OnComponentEndOverlap(Sphere)
  (params (OverlappedComponent :type Primitive%20Component%20Object%20Reference) (OtherActor :type Actor%20Object%20Reference) (OtherComp :type Primitive%20Component%20Object%20Reference) (OtherBodyIndex :type Integer))
  ;[0 0 0 1 35] Stop Overlap go back to Idle
  (if (not (Collision|IsOverlappingActor (Variables|Default|GetTPCref) :!class /Script/Engine.Actor))
    (AI|AIMoveTo self (Variables|Default|GetWorldLocation) 0 5.0 false
      (:OnSuccess
        (bind _asabp_mutant (Utilities|Casting|CastToABP_Mutant (Variables|Default|GetAnimInstance)))
        (Variables|/Game/Characters/NPC/ABP_Mutant.ABP_Mutant_C|SetbIsWalking _asabp_mutant false)
        (Variables|/Game/Characters/NPC/ABP_Mutant.ABP_Mutant_C|SetbIsReaction _asabp_mutant false)))))

(event OnComponentBeginOverlap(RhandBoxCollision)
  (params (OverlappedComponent :type Primitive%20Component%20Object%20Reference) (OtherActor :type Actor%20Object%20Reference) (OtherComp :type Primitive%20Component%20Object%20Reference) (OtherBodyIndex :type Integer) (bFromSweep :type Boolean) (SweepResult :type Hit%20Result%20Structure%20%28by%20ref%29))
  (bind _asbp_third_person_character (Utilities|Casting|CastToBP_ThirdPersonCharacter OtherActor))
  (Variables|Default|SetbIsOverlapCapsule true)
  (Development|PrintString "overlap")
  (if (Variables|Default|GetIsPunchingNPC)
    (Development|PrintString "Punching")
    (if (Class|PrimitiveComponent|IsOverlappingComponent (Variables|/Script/Engine.Character|GetCapsuleComponent _asbp_third_person_character) (Variables|Default|GetRhand%20Box%20Collision))
      (bind _asbp_third_person_character_2 (Utilities|Casting|CastToBP_ThirdPersonCharacter OtherActor))
      (Variables|/Game/ThirdPerson/Blueprints/BP_ThirdPersonCharacter.BP_ThirdPersonCharacter_C|SetPv _asbp_third_person_character_2 (- (Variables|/Game/ThirdPerson/Blueprints/BP_ThirdPersonCharacter.BP_ThirdPersonCharacter_C|GetPv _asbp_third_person_character_2) 1e+01))
      (if (<= (Variables|/Game/ThirdPerson/Blueprints/BP_ThirdPersonCharacter.BP_ThirdPersonCharacter_C|GetPv _asbp_third_person_character_2) 0.0)
        (Development|PrintString "Hello")))))

(event OnComponentBeginOverlap(Sphere)
  (params (OverlappedComponent :type Primitive%20Component%20Object%20Reference) (OtherActor :type Actor%20Object%20Reference) (OtherComp :type Primitive%20Component%20Object%20Reference) (OtherBodyIndex :type Integer) (bFromSweep :type Boolean) (SweepResult :type Hit%20Result%20Structure%20%28by%20ref%29))
  ;[0 0 0 1 35] Overlap Sphere NPC start walking toward TPC/Punching TPC
  (if (Collision|IsOverlappingActor (Variables|Default|GetTPCref) :!class /Script/Engine.Actor)
    (Utilities|FlowControl|Sequence
      (:then_0
        (bind _asabp_mutant (Utilities|Casting|CastToABP_Mutant (Variables|Default|GetAnimInstance)))
        (Variables|/Game/Characters/NPC/ABP_Mutant.ABP_Mutant_C|SetbIsWalking _asabp_mutant true)
        (Variables|/Game/Characters/NPC/ABP_Mutant.ABP_Mutant_C|SetbIsReaction _asabp_mutant false)
        (AI|AIMoveTo self "0, 0, 0" (Variables|Default|GetTPCref) 5.0 false)))))

(event Custom|Drop%20Loot
  (bind _returnvalue (Transformation|GetActorLocation))
  ;[0 0 0 1 35] Drop Loot when ennemy dies
  (bind _outhit (Collision|LineTraceByChannel _returnvalue (- _returnvalue "0,0,200.000000") "TraceTypeQuery1" false (Utilities|Array|MakeArray (Game|GetPlayerCharacter 0)) "None"))
  (Game|SpawnActorfromClass (Utilities|Select :Index (Math|Random|RandomInteger 2) :Option%200 "/Game/InventorySystem/ProjectExample/Blueprints/BP_Pickup.BP_Pickup_C" :Option%201 "/Game/NFT/BP_NFT.BP_NFT_C") (Math|Transform|MakeTransform (.RandomLocation (AI|Navigation|GetRandomReachablePointinRadius (.Location (Collision|BreakHitResult _outhit)) 2e+02 0 0)) (Math|Rotator|MakeRotator 0.0 0.0 (Math|Random|RandomFloatinRange 0.0 3.6e+02))) "AdjustIfPossibleButAlwaysSpawn" 0 0))

(event Custom|ByeLife
  ;[0 0 0 1 35] NPC Loosing Life and Dying
  (Variables|Default|SetPV (- (Variables|Default|GetPV) 1e+01))
  (if (<= (Variables|Default|GetPV) 0.0)
    (bind _asabp_mutant (Utilities|Casting|CastToABP_Mutant (Variables|Default|GetAnimInstance)))
    (Variables|/Game/Characters/NPC/ABP_Mutant.ABP_Mutant_C|SetbIsDying _asabp_mutant true)
    (Components|Movement|StopMovementImmediately (Variables|Character|GetCharacterMovement))
    (Utilities|FlowControl|Delay 5.0)
    (CallFunction|DropLoot)
    (Actor|DestroyActor)))

(event EventBeginPlay
  ;[0 0 0 1 35] Begin Play
  (Components|Animation|PlayAnimation (Variables|Character|GetMesh) "/Game/Characters/NPC/Animation/Mutant_Breathing_Idle.Mutant_Breathing_Idle" true)
  (bind _asbp_third_person_character (Utilities|Casting|CastToBP_ThirdPersonCharacter (Game|Player|GetPlayerPawn 0)))
  (Variables|Default|SetTPCref _asbp_third_person_character)
  (Variables|Default|SetWorldLocation (Transformation|GetWorldLocation (Variables|Character|GetMesh)))
  (Class|SkeletalMeshComponent|SetAnimClass (Variables|Character|GetMesh) (Utilities|Select :Index (Variables|Default|GetNPCChoice) :NewEnumerator0 "/Game/Characters/NPC/ABP_Mutant.ABP_Mutant_C" :NewEnumerator1 "/Game/Characters/Mannequins/Animations/ABP_Quinn.ABP_Quinn_C" :NewEnumerator2 "/Game/Characters/Mannequins/Animations/ABP_Manny.ABP_Manny_C"))
  (Variables|Default|SetAnimInstance (Components|SkeletalMesh|GetAnimInstance (Variables|Character|GetMesh))))

(event EventTick
  (params (DeltaSeconds :type Float%20%28single-precision%29))
  (bind _animinstance (Variables|Default|GetAnimInstance))
  ;[0 0 0 1 35] Overlap Sphere NPC start walking toward TPC/Punching TPC
  (if (< (Math|Float|Round (Transformation|GetDistanceTo (Variables|Default|GetTPCref) self)) 200)
    (Utilities|FlowControl|DoOnce false :!label _label
      (:Completed
        (Variables|Default|SetbIsDistance true)
        (bind _asabp_mutant (Utilities|Casting|CastToABP_Mutant _animinstance))
        (Variables|/Game/Characters/NPC/ABP_Mutant.ABP_Mutant_C|SetbIsWalking _asabp_mutant true)
        (Animation|Montage|MontagePlay (Variables|Default|GetAnimInstance) "/Game/Characters/NPC/Animation/Mutant_Punch_Montage.Mutant_Punch_Montage" 1.0 "MontageLength" 0.0 true)
        (AI|AIMoveTo self "0, 0, 0" (Variables|Default|GetTPCref) 5.0 false
          (:then
            (Variables|Default|SetIsPunchingNPC true)))))
    (else
      (Utilities|FlowControl|Sequence
        (:then_0
          (goto _label Reset))
        (:then_1
          (Variables|Default|SetbIsDistance false)
          (bind _asabp_mutant_2 (Utilities|Casting|CastToABP_Mutant _animinstance))
          (Variables|/Game/Characters/NPC/ABP_Mutant.ABP_Mutant_C|SetbIsPunching _asabp_mutant_2 false)
          (Variables|Default|SetIsPunchingNPC false))))))

(fn ConstructionScript
  (Class|SkinnedMeshComponent|SetSkeletalMesh (Variables|Character|GetMesh) (Utilities|Array|Get(acopy) (Variables|Default|GetListeNPC) (Math|Conversions|ToInteger(Byte) (Variables|Default|GetNPCChoice))) true))